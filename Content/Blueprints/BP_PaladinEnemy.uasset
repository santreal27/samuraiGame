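; BP_PaladinEnemy is a melee enemy that chases the player on sight and attacks with a sword slash montage.
; PawnSensing starts an AI MoveTo, whose success plays the slash while movement is deactivated.
; Sword trigger events run a looping timer that box-traces at the sword's collision box to damage BP_MariaCharacter.
; Incoming damage passes a DoOnce cooldown, and zero health plays a death montage before destroying the actor.
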(event OnSeePawn(PawnSensing)
  (params (Pawn :type Pawn%20Object%20Reference))
  (Variables|Default|SetIsSeeingPlayer true)
  (CallFunction|FollowPlayer))

(event Custom|FollowPlayer
  (Variables|Default|SetCanAttack true)
  (if (Variables|Default|GetIsSeeingPlayer)
    (AI|AIMoveTo self "0, 0, 0" (Game|GetPlayerCharacter 0) 5.0 false
      (:OnSuccess
        (if (Variables|Default|GetCanAttack)
          (Variables|Default|SetCanAttack false)
          (Variables|Default|SetIsAttacking true)
          (Animation|Montage|PlayMontage (Variables|Character|GetMesh) "/Game/PaladinCharacter/Animations/AM_Slash.AM_Slash"
            (:then
              (Components|Activation|Deactivate (Variables|Character|GetCharacterMovement)))
            (:OnCompleted
              (Components|Activation|Activate (Variables|Character|GetCharacterMovement) false)
              (Variables|Default|SetIsAttacking false))))))
    (else
      (Variables|Default|SetIsSeeingPlayer false))))

(event Custom|OnDeath
  ;[1 1 1] OnDeathEvent
  (Components|Activation|Deactivate (Variables|Default|GetPawnSensing))
  (Components|Activation|Deactivate (Variables|Character|GetCharacterMovement))
  (Animation|StopAnimMontage "/Game/PaladinCharacter/Animations/AM_Slash.AM_Slash")
  (bind _returnvalue (Animation|PlayAnimMontage "/Game/PaladinCharacter/Animations/AM_PaladinDeath.AM_PaladinDeath" 1.0 "None"))
  (Utilities|FlowControl|Delay _returnvalue)
  (Actor|DestroyActor))

(event Custom|TriggerSword
  ;[1 1 1] Trigger Sword Event
  (bind _returnvalue (Utilities|Time|SetTimerbyEvent (delegate Custom|SwordLineTrace) 0.01 true))
  (Variables|Default|SetTriggerSwordEvent _returnvalue))

(event Custom|SwordLineTrace
  (bind _swordboxcollision (Variables|Default|GetSwordBoxCollision))
  (bind _returnvalue (Transformation|GetWorldLocation _swordboxcollision))
  ;[1 1 1] Trigger Sword Event
  (bind (_outhit _returnvalue_2) (Collision|BoxTraceByChannel _returnvalue _returnvalue (Components|Box|GetScaledBoxExtent _swordboxcollision) (Transformation|GetWorldRotation _swordboxcollision) "TraceTypeQuery1" false 0 "None"))
  (if _returnvalue_2
    (bind _asbp_maria_character (Utilities|Casting|CastToBP_MariaCharacter (.HitActor (Collision|BreakHitResult _outhit))))
    (Game|Damage|ApplyDamage _asbp_maria_character (Variables|Default|GetDamage) 0 0)))

(event Custom|StopTriggerSword
  ;[1 1 1] Trigger Sword Event
  (Utilities|Time|ClearandInvalidateTimerbyHandle (Variables|Default|GetTriggerSwordEvent)))

(event EventBeginPlay
  (Variables|Default|SetCurrentHealth (Variables|Default|GetMaxHealth)))

(event Game|Damage|EventAnyDamage
  (params (Damage :type Float%20%28single-precision%29) (DamageType :type Damage%20Type%20Object%20Reference) (InstigatedBy :type Controller%20Object%20Reference) (DamageCauser :type Actor%20Object%20Reference))
  ;[1 1 1] Receiving Damage
  (Utilities|FlowControl|DoOnce false :!label _label
    (:Completed
      (CallFunction|TakeDamage Damage)
      (if (<= (Variables|Default|GetCurrentHealth) 0.0)
        (CallFunction|OnDeath)
        (else
          (Utilities|FlowControl|Delay 1.0)
          (goto _label Reset))))))

(event EventTick
  (params (DeltaSeconds :type Float%20%28single-precision%29))
  (if (not (Variables|Default|GetIsSeeingPlayer))
    (Components|Movement|StopMovementImmediately (Variables|Character|GetCharacterMovement))))

(fn ConstructionScript)

(fn TakeDamage
  (params (Damage :type Float%20%28double-precision%29))
  (Variables|Default|SetCurrentHealth (- (Variables|Default|GetCurrentHealth) Damage))
  (Audio|PlaySoundatLocation "/Game/Audio/DamageSound.DamageSound" (Transformation|GetActorLocation) "0, 0, 0" 1.0 1.0 0.0 0 0 0 0))