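; BP_EnemyUnit is an enemy with health that is damaged by contact with an attacking BP_MariaCharacter.
; CurrentHealth starts at MaxHealth on BeginPlay.
; On actor overlap it casts to the Maria character and, if IsAttacking is set, passes that character's Damage to TakeDamage and plays a damage sound at its location.
; TakeDamage only subtracts from CurrentHealth, with no clamp or death handling.
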(event EventBeginPlay
  (Variables|Default|SetCurrentHealth (Variables|Default|GetMaxHealth)))

(event EventTick
  (params (DeltaSeconds :type Float%20%28single-precision%29)))

(event Collision|EventActorBeginOverlap
  (params (OtherActor :type Actor%20Object%20Reference))
  (bind _asbp_maria_character (Utilities|Casting|CastToBP_MariaCharacter OtherActor))
  (if (Variables|/Game/Blueprints/BP_MariaCharacter.BP_MariaCharacter_C|GetIsAttacking _asbp_maria_character)
    (CallFunction|TakeDamage (Variables|/Game/Blueprints/BP_MariaCharacter.BP_MariaCharacter_C|GetDamage _asbp_maria_character))
    (Audio|PlaySoundatLocation "/Game/Audio/DamageSound.DamageSound" (Transformation|GetActorLocation) "0, 0, 0" 1.0 1.0 0.0 0 0 0 0)))

(fn ConstructionScript)

(fn TakeDamage
  (params (Damage :type Float%20%28double-precision%29))
  (Variables|Default|SetCurrentHealth (- (Variables|Default|GetCurrentHealth) Damage)))